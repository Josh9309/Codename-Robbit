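; RobbitCharacter is the player character Blueprint, handling movement, jumping, camera look and creation of the HUD widget.
; Movement projects the mesh's right vector for forward and negated forward vector for strafing onto the ground plane, scaled by speed and delta time.
; Horizontal look yaws the mesh, while vertical look rolls CameraFocusPoint.
; IsGrounded gates both Jump and a per-tick vertical movement input scaled by Gravity, but is never set here.
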(event EventBeginPlay
  ;[1 1 1] For Crosshair HUD
  (CallFunction|CreateHUD))

(event Collision|EventActorBeginOverlap
  (params (OtherActor :type Actor%20Object%20Reference)))

(event EventTick
  (params (DeltaSeconds :type Float%20%28single-precision%29))
  ;[1 1 1] Applies Gravity
  (if (Variables|Default|GetIs_Grounded)
    (Pawn|Input|AddMovementInput "0.000000, 0,1.000000" (* (Variables|Default|Getgravity) (Utilities|Time|GetWorldDeltaSeconds)) false)))

(event Input|ActionEvents|InputActionJump
  (params (Key :type Key%20Structure))
  ;[1 1 1] Jump Logic
  (:Pressed
    (if (Variables|Default|GetIs_Grounded)
      (Character|Jump))))

(event Input|AxisEvents|InputAxisMoveForward
  (params (AxisValue :type Float%20%28single-precision%29))
  ;[1 1 1] Move Forward/Backward Input
  (Development|PrintString (Utilities|String|ToString(Float) AxisValue))
  (Pawn|Input|AddMovementInput (Math|Vector|ProjectVectorontoPlane (Math|Vector|GetRightVector (Variables|Character|GetMesh)) "0,0.000000,1.000000") (* AxisValue (Variables|Default|GetRobbit%20Movement%20Speed) (Utilities|Time|GetWorldDeltaSeconds)) false))

(event Input|AxisEvents|InputAxisMoveRight
  (params (AxisValue :type Float%20%28single-precision%29))
  ;[1 1 1] Strafe Left/Right Logic
  (Pawn|Input|AddMovementInput (Math|Vector|ProjectVectorontoPlane (* (Math|Vector|GetForwardVector (Variables|Character|GetMesh)) -1.0) "0, 0,1.000000") (* AxisValue (Variables|Default|GetRobbit%20Movement%20Speed) (Utilities|Time|GetWorldDeltaSeconds)) false))

(event Input|AxisEvents|InputAxisCameraHorizontal
  (params (AxisValue :type Float%20%28single-precision%29))
  ;[1 1 1] Rotates Camera
  (Transformation|SetRelativeRotation (Variables|Character|GetMesh) (Math|Rotator|CombineRotators (Variables|/Script/Engine.SceneComponent|GetRelativeRotation (Variables|Character|GetMesh)) (Math|Rotator|MakeRotator 0.0 0.0 (* (Utilities|Time|GetWorldDeltaSeconds) (Variables|Default|GetCam%20Sensitivity%20X) AxisValue))) false false))

(event Input|AxisEvents|InputAxisCameraVertical
  (params (AxisValue :type Float%20%28single-precision%29))
  (bind _camera_focus_point (Variables|Default|GetCamera%20Focus%20Point))
  ;[1 1 1] Rotates Camera
  (Transformation|SetRelativeRotation _camera_focus_point (Math|Rotator|CombineRotators (Variables|/Script/Engine.SceneComponent|GetRelativeRotation _camera_focus_point) (Math|Rotator|MakeRotator (* AxisValue (Variables|Default|GetCam%20Sensitivity%20Y) (Utilities|Time|GetWorldDeltaSeconds)) 0.0 0.0)) false false))

(fn ConstructionScript)

(fn CreateHUD
  (bind _returnvalue (UserInterface|CreateWidget "/Game/Blueprints/UI/HUD.HUD_C"))
  (UserInterface|Viewport|AddtoViewport _returnvalue 0))