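; RobbitPawn is a player pawn Blueprint with forward/backward movement, camera control and a jump, all driven by input.
; Movement follows the camera's forward vector flattened onto the ground plane.
; Horizontal look yaws the whole actor, while vertical look rotates CameraFocusPoint through its roll axis.
; Gravity and jump both use vertical AddMovementInput gated on IsGrounded, which this graph never sets; a JumpForce velocity calculation sits unused.
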(event EventBeginPlay)

(event Collision|EventActorBeginOverlap
  (params (OtherActor :type Actor%20Object%20Reference)))

(event EventTick
  (params (DeltaSeconds :type Float%20%28single-precision%29))
  ;[1 1 1] Applies Gravity
  (if (Variables|Default|GetIs_Grounded)
    (Pawn|Input|AddMovementInput "0.000000, 0,1.000000" (* (Variables|Default|Getgravity) (Utilities|Time|GetWorldDeltaSeconds)) false)))

(event Input|ActionEvents|InputActionJump
  (params (Key :type Key%20Structure))
  ;[1 1 1] Jump Logic
  (:Pressed
    (if (Variables|Default|GetIs_Grounded)
      (Pawn|Input|AddMovementInput "0, 0,100.000000" 1.0 true))))

(event Input|AxisEvents|InputAxisMoveForward
  (params (AxisValue :type Float%20%28single-precision%29))
  ;[1 1 1] Move Forward/Backward Input
  (Pawn|Input|AddMovementInput (Math|Vector|ProjectVectorontoPlane (Math|Vector|GetForwardVector (Variables|Default|GetRobbit%20Camera)) "0,0.000000,1.000000") (* AxisValue (Variables|Default|GetRobbit%20Movement%20Speed) (Utilities|Time|GetWorldDeltaSeconds)) false))

(event Input|AxisEvents|InputAxisCameraHorizontal
  (params (AxisValue :type Float%20%28single-precision%29))
  ;[1 1 1] Rotates Camera
  (Transformation|SetActorRotation (Math|Rotator|CombineRotators (Transformation|GetActorRotation) (Math|Rotator|MakeRotator 0.0 0.0 (* (Utilities|Time|GetWorldDeltaSeconds) (Variables|Default|GetCam%20Sensitivity%20X) AxisValue)))))

(event Input|AxisEvents|InputAxisCameraVertical
  (params (AxisValue :type Float%20%28single-precision%29))
  (bind _camera_focus_point (Variables|Default|GetCamera%20Focus%20Point))
  ;[1 1 1] Rotates Camera
  (Transformation|SetRelativeRotation _camera_focus_point (Math|Rotator|CombineRotators (Variables|/Script/Engine.SceneComponent|GetRelativeRotation _camera_focus_point) (Math|Rotator|MakeRotator (* AxisValue (Variables|Default|GetCam%20Sensitivity%20Y) (Utilities|Time|GetWorldDeltaSeconds)) 0.0 0.0)) false false))

(fn ConstructionScript)